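; BP_HideLocker is a hiding spot that the third-person character enters and exits with the Interact input.
; Overlapping its box shows a prompt widget, enables input and opens a gate; leaving reverses all three.
; ToggleHide flips the character's visibility and collision and blends the camera between character and locker.
; A short delay after each toggle re-enables input and reopens the gate, even if an end overlap closed it.
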(event OnComponentBeginOverlap(Box)
  (params (OverlappedComponent :type Primitive%20Component%20Object%20Reference) (OtherActor :type Actor%20Object%20Reference) (OtherComp :type Primitive%20Component%20Object%20Reference) (OtherBodyIndex :type Integer) (bFromSweep :type Boolean) (SweepResult :type Hit%20Result%20Structure%20%28by%20ref%29))
  (Utilities|FlowControl|Sequence
    (:then_0
      (bind _asbp_third_person_character (Utilities|Casting|CastToBP_ThirdPersonCharacter OtherActor))
      (Variables|Default|SetCharRef _asbp_third_person_character)
      (Input|EnableInput (Game|GetPlayerController 0))
      (Utilities|FlowControl|Gate true) ; enters at Open
    )
    (:then_1
      (Rendering|SetVisibility (Variables|Default|GetWidget) true false))))

(event OnComponentEndOverlap(Box)
  (params (OverlappedComponent :type Primitive%20Component%20Object%20Reference) (OtherActor :type Actor%20Object%20Reference) (OtherComp :type Primitive%20Component%20Object%20Reference) (OtherBodyIndex :type Integer))
  (bind _returnvalue (Game|GetPlayerController 0))
  (Utilities|FlowControl|Sequence
    (:then_0
      (Utilities|Casting|CastToBP_ThirdPersonCharacter OtherActor)
      (Input|DisableInput _returnvalue)
      (Utilities|FlowControl|Gate true) ; enters at Close
    )
    (:then_1
      (Rendering|SetVisibility (Variables|Default|GetWidget) false false))))

(event Input|ActionEvents|InputActionInteract
  (params (Key :type Key%20Structure :default "None"))
  (:Pressed
    (Utilities|FlowControl|Gate true :!label _label
      (:Exit
        (CallFunction|ToggleHide)
        (Utilities|FlowControl|Delay 0.2)
        (Input|EnableInput (Game|GetPlayerController 0))
        (goto _label Open)))))

(fn ConstructionScript
  (|CallParentFunction))

(fn ToggleHide
  (bind _returnvalue (Game|GetPlayerController 0))
  (bind _charref (Variables|Default|GetCharRef))
  (if (Variables|Default|GetisHiding)
    (Variables|Default|SetisHiding false)
    (Rendering|SetActorHiddenInGame _charref false)
    (Collision|SetActorEnableCollision _charref true)
    (Game|Player|SetViewTargetwithBlend _returnvalue _charref 0.6 "VTBlend_Linear" 0.0 false)
    (else
      (Variables|Default|SetisHiding true)
      (Rendering|SetActorHiddenInGame _charref true)
      (Collision|SetActorEnableCollision _charref false)
      (Game|Player|SetViewTargetwithBlend _returnvalue self 0.6 "VTBlend_Linear" 0.0 false))))