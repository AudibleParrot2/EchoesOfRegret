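; BP_HighLightFlicker is a spotlight Blueprint that flickers continuously at irregular intervals.
; The construction script sets the SpotLight to its base Intensity.
; From BeginPlay, a self-looping retriggerable delay waits a random time between MinTime and MaxTime.
; A FlipFlop then alternates between a random dim level, from a hardcoded floor to MinFlicker, and a random bright level, from MinFlicker to Intensity.
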(event EventBeginPlay
  (bind _minflicker (Variables|Default|GetMinFlicker))
  (bind _spotlight (Variables|Default|GetSpotLight))
  (Utilities|FlowControl|RetriggerableDelay (Math|Random|RandomFloatinRange (Variables|Default|GetMinTime) (Variables|Default|GetMaxTime)) :!label _label)
  (Utilities|FlowControl|FlipFlop
    (:A
      (Rendering|Components|Light|SetIntensity _spotlight (Math|Random|RandomFloatinRange 5e+03 _minflicker))
      (goto _label))
    (:B
      (Rendering|Components|Light|SetIntensity _spotlight (Math|Random|RandomFloatinRange _minflicker (Variables|Default|GetIntensity)))
      (goto _label))))

(fn ConstructionScript
  (Rendering|Components|Light|SetIntensity (Variables|Default|GetSpotLight) (Variables|Default|GetIntensity)))