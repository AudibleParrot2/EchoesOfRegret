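; A locked door actor that opens only after its key has been picked up.
; A box overlap shows and hides a prompt widget near the door, and a key pickup event sets a HasKey flag.
; Interact checks that flag, then disables the box collision and plays a timeline that swings the door's yaw open, or prints a need-a-key message otherwise.
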(event OnComponentBeginOverlap(Box)
  (params (OverlappedComponent :type Primitive%20Component%20Object%20Reference) (OtherActor :type Actor%20Object%20Reference) (OtherComp :type Primitive%20Component%20Object%20Reference) (OtherBodyIndex :type Integer) (bFromSweep :type Boolean) (SweepResult :type Hit%20Result%20Structure%20%28by%20ref%29))
  (Rendering|SetVisibility (Variables|Default|GetWidget) true false))

(event OnComponentEndOverlap(Box)
  (params (OverlappedComponent :type Primitive%20Component%20Object%20Reference) (OtherActor :type Actor%20Object%20Reference) (OtherComp :type Primitive%20Component%20Object%20Reference) (OtherBodyIndex :type Integer))
  (Rendering|SetVisibility (Variables|Default|GetWidget) false false))

(event EventOnKeyPickup
  (Variables|Default|SethasKey true))

(event EventInteract
  (bind _door (Variables|Default|GetDoor))
  (bind _relativerotation (Variables|/Script/Engine.SceneComponent|GetRelativeRotation _door))
  (if (Variables|Default|GethasKey)
    (Collision|SetCollisionEnabled (Variables|Default|GetBox) "NoCollision")
    (bind _doorfloat (Timeline|OpenLockedDoor Play)
      (:Update
        (Transformation|SetRelativeRotation _door (Math|Rotator|MakeRotator (.roll _relativerotation) (.pitch _relativerotation) (Math|Float|Lerp 0.0 -1.2e+02 _doorfloat)) false false)))
    (else
      (Development|PrintString "Need a Key!!"))))

(fn ConstructionScript)