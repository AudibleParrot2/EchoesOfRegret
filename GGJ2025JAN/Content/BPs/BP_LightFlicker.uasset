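; BP_LightFlicker is a Blueprint that makes a spot light flicker at irregular intervals during play.
; The construction script sets the base Intensity, then BeginPlay starts an endless loop with a retriggerable delay of random length between MinTime and MaxTime.
; After each delay a FlipFlop alternates between a random dim value up to MinFlicker and a random brighter value between MinFlicker and Intensity.
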(event EventBeginPlay
  (bind _spotlight (Variables|Default|GetSpotLight))
  (bind _minflicker (Variables|Default|GetMinFlicker))
  (Utilities|FlowControl|RetriggerableDelay (Math|Random|RandomFloatinRange (Variables|Default|GetMinTime) (Variables|Default|GetMaxTime)) :!label _label)
  (Utilities|FlowControl|FlipFlop
    (:A
      (Rendering|Components|Light|SetIntensity _spotlight (Math|Random|RandomFloatinRange 0.0 _minflicker))
      (goto _label))
    (:B
      (Rendering|Components|Light|SetIntensity _spotlight (Math|Random|RandomFloatinRange _minflicker (Variables|Default|GetIntensity)))
      (goto _label))))

(fn ConstructionScript
  (Rendering|Components|Light|SetIntensity (Variables|Default|GetSpotLight) (Variables|Default|GetIntensity)))